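; Collectible pickup Blueprint, apparently a totem, built around a Collision component.
; When that component begins an overlap, it only sets the Collectible01HIT flag to true.
; A disconnected chain would guard with HIT, increment TotemsCollected on the cast overlapping actor, then destroy itself after a short delay, but it never runs.
; The actor-level overlap event and construction script are empty.
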(event `self.ReceiveActorBeginOverlap`
  (params (OtherActor :type "Actor Object Reference"))
  ;[1 1 1] Totems Collected
)

(event `self.collision.OnComponentBeginOverlap`
  (params (OverlappedComponent :type "PrimitiveComponent Object Reference") (OtherActor :type "Actor Object Reference") (OtherComp :type "PrimitiveComponent Object Reference") (OtherBodyIndex :type Integer) (bFromSweep :type Boolean) (SweepResult :type "HitResult Structure (by ref)"))
  ;[1 1 1] Check Boolean
  (set `self.collectible01HIT` true))

(fn `UserConstructionScript`)