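; Collectible totem actor that the Eiko player character picks up by overlapping it.
; On actor overlap it sets a one-shot HIT flag before casting to EikoPlayerCharacter, so any first overlapping actor consumes it.
; A successful cast increments the character's TotemsCollected count, then destroys the totem after a short delay.
; A separate Collision component overlap sets a Collectible01HIT flag, which this graph never reads.
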(event `self.ReceiveActorBeginOverlap`
  (params (OtherActor :type "Actor Object Reference"))
  ;[1 1 1] Totems Collected
  (if (not (`self.HIT`))
    (set `self.HIT` true)
    (bind _aseiko_player_character (cast `/Game/EikoPlayerCharacterBP/Blueprints/EikoPlayerCharacter` OtherActor))
    (set `/Game/EikoPlayerCharacterBP/Blueprints/EikoPlayerCharacter.TotemsCollected` (+ (`/Game/EikoPlayerCharacterBP/Blueprints/EikoPlayerCharacter.TotemsCollected` _aseiko_player_character) 1) _aseiko_player_character)
    (`KismetSystemLibrary.Delay` 0.2)
    (`self.K2_DestroyActor`)))

(event `self.collision.OnComponentBeginOverlap`
  (params (OverlappedComponent :type "PrimitiveComponent Object Reference") (OtherActor :type "Actor Object Reference") (OtherComp :type "PrimitiveComponent Object Reference") (OtherBodyIndex :type Integer) (bFromSweep :type Boolean) (SweepResult :type "HitResult Structure (by ref)"))
  ;[1 1 1] Check Boolean
  (set `self.collectible01HIT` true))

(fn `UserConstructionScript`)